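; Game mode Blueprint for the medium labyrinth level, supplying level-specific placement data to its parent game mode.
; On BeginPlay it runs SetParentVariables before the parent's BeginPlay, filling inherited transforms for trashcan, spider and fire spawn events plus escape and distractor signs.
; The fire transform, identical to the trashcan's, sits on a Sequence pin after the one wired to the Return node.
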(event EventBeginPlay
  (CallFunction|SetParentVariables)
  (|CallParentFunction))

(event EventTick
  (params (DeltaSeconds :type Float%20%28single-precision%29)))

(fn ConstructionScript
  (|CallParentFunction))

(fn SetParentVariables
  ;[1 1 1] Set the variables of the parent blueprint which depend on the level
  (Utilities|FlowControl|Sequence
    (:then_0
      (Variables|Default|SetTrashcanSpawnEventTransform (Math|Transform|MakeTransform "-260.000000,1420.000000,51.000000" "0.000000,0.000000,90.000000" "5.000000,5.000000,5.000000")))
    (:then_1
      (Variables|Default|SetSpiderSpawnEventTransform (Math|Transform|MakeTransform "-260.000000,1410.000000,51.000000" "0.000000,-180.000000,0.000000" "1.000000,1,1")))
    (:then_2
      (Variables|Default|SetEscapesignSpawnTransform1 (Math|Transform|MakeTransform "-650.000000,210.000000,370.000000" "0.000000,90.000000,90.000000" "3.000000,3.000000,3.000000")))
    (:then_3
      (Variables|Default|SetEscapesignSpawnTransform2 (Math|Transform|MakeTransform "-520.000000,-1450.000000,370.000000" "0.000000,0.000000,90.000000" "3.000000,3.000000,3.000000")))
    (:then_4
      (Variables|Default|SetEscapesignSpawnTransform3 (Math|Transform|MakeTransform "100.000000,-10.000000,370.000000" "0.000000,0.000000,90.000000" "3.000000,3.000000,3.000000")))
    (:then_5
      (Variables|Default|SetDistractorsignSpawnTransform1 (Math|Transform|MakeTransform "790.000000,-370.000000,370.000000" "0.000000,-180.000000,90.000000" "3.000000,3.000000,3.000000")))
    (:then_6
      (Variables|Default|SetDistractorsignSpawnTransform2 (Math|Transform|MakeTransform "1450.000000,-680.000000,370.000000" "0.000000,90.000000,90.000000" "3.000000,3.000000,3.000000")))
    (:then_7
      (return))
    (:then_8
      (Variables|Default|SetFireSpawnEventTransform (Math|Transform|MakeTransform "-260.000000,1420.000000,51.000000" "0.000000,0.000000,90.000000" "5.000000,5.000000,5.000000")))))