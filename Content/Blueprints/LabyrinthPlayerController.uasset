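; Player controller for the labyrinth game that handles input for toggling alarm mode and launching the medium level.
; The alarm input flips AlarmMode on the labyrinth game mode, then writes the new value into a freshly created AlarmModeSaver and saves it to a slot.
; The level input sets NewLevel to MediumLevel, which StartLevel prints and opens by name.
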(event EventBeginPlay)

(event EventTick
  (params (DeltaSeconds :type Float%20%28single-precision%29)))

(event Input|ActionEvents|InputActionEnableAlarmMode
  (params (Key :type Key%20Structure :default "AnyKey"))
  (:Pressed
    (CallFunction|SwitchAlarmMode)))

(event Input|ActionEvents|InputActionStartMediumLevel
  (params (Key :type Key%20Structure :default "AnyKey"))
  (:Pressed
    (Variables|Default|SetNewLevel (Variables|Default|GetMediumLevel))
    (CallFunction|StartLevel)))

(fn ConstructionScript)

(fn SwitchAlarmMode
  (bind _aslabyrinth_game_mode_blueprint (Utilities|Casting|CastToLabyrinthGameModeBlueprint (Game|GetGameMode))
    (:then
      ;[1 1 1] Change AlarmMode
      (Variables|Default|SetGameMode _aslabyrinth_game_mode_blueprint)
      (Development|PrintString "CHANGE ALARM MODE" false)
      (Variables|/Game/Blueprints/LabyrinthGameModeBlueprint.LabyrinthGameModeBlueprint_C|SetAlarmMode (Variables|Default|GetGameMode) (not (Variables|/Game/Blueprints/LabyrinthGameModeBlueprint.LabyrinthGameModeBlueprint_C|GetAlarmMode (Variables|Default|GetGameMode))))
      (bind _returnvalue (SaveGame|CreateSaveGameObject "/Game/Blueprints/AlarmModeSaver.AlarmModeSaver_C"))
      (bind _asalarm_mode_saver (Utilities|Casting|CastToAlarmModeSaver _returnvalue)
        (:then
          (bind _output_get (Variables|Default|SetAlarmSave _asalarm_mode_saver))
          (Variables|/Game/Blueprints/AlarmModeSaver.AlarmModeSaver_C|SetIsAlarmModeOn _output_get (Variables|/Game/Blueprints/LabyrinthGameModeBlueprint.LabyrinthGameModeBlueprint_C|GetAlarmMode (Variables|Default|GetGameMode)))
          (SaveGame|SaveGametoSlot (Variables|Default|GetAlarmSave) (Variables|Default|GetAlarmModeSave) (Variables|Default|GetAlarmSaveId)))
        (:CastFailed
          _)))
    (:CastFailed
      _))
  (return))

(fn StartLevel
  (bind _newlevel (Variables|Default|GetNewLevel))
  ;[1 1 1] Start Medium Level
  (Development|PrintString (Utilities|String|Append "Start" (Utilities|String|ToString(Name) _newlevel)) false)
  (Game|OpenLevel(byName) _newlevel false)
  (return))