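; Game mode for a labyrinth level that sets up signs, an alarm and a random object on BeginPlay.
; It reads toggles from LabyrinthGameInstance to spawn escape signs, distractor signs (phone, ladder, fire extinguisher) at preset transforms, and a fire alarm sound after a delay.
; Independently of the toggles, it spawns one random object: a trashcan, spider or fire.
; Debug text reports each toggle's state.
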(event EventTick
  (params (DeltaSeconds :type Float%20%28single-precision%29)))

(event EventBeginPlay
  (Utilities|FlowControl|Sequence
    (:then_0
      ;[1 1 1] Get Variables from LabyrinthGameInstance
      (bind _aslabyrinth_game_instance (Utilities|Casting|CastToLabyrinthGameInstance (Game|GetGameInstance))
        (:then
          (Utilities|FlowControl|Sequence
            (:then_0
              (if (Variables|/Game/Blueprints/LabyrinthGameInstance.LabyrinthGameInstance_C|GetEscapeSignsEnabled _aslabyrinth_game_instance)
                (Development|PrintText "Escape Signs ON!" false)
                ;[1 1 1] Spawn Escape Signs
                (Utilities|FlowControl|Sequence
                  (:then_0
                    (Game|SpawnActorfromClass "/Game/Blueprints/EscapeBlueprint.EscapeBlueprint_C" (Variables|Default|GetEscapesignSpawnTransform1) "Undefined" 0 0))
                  (:then_1
                    (Game|SpawnActorfromClass "/Game/Blueprints/EscapeBlueprint.EscapeBlueprint_C" (Variables|Default|GetEscapesignSpawnTransform2) "Undefined" 0 0))
                  (:then_2
                    (Game|SpawnActorfromClass "/Game/Blueprints/EscapeBlueprint.EscapeBlueprint_C" (Variables|Default|GetEscapesignSpawnTransform3) "Undefined" 0 0)))
                (else
                  (Development|PrintText "Escape Signs OFF!" false))))
            (:then_1
              (if (Variables|/Game/Blueprints/LabyrinthGameInstance.LabyrinthGameInstance_C|GetDistractingSignsEnabled _aslabyrinth_game_instance)
                (Development|PrintText "Distracting Signs ON!" false)
                ;[1 1 1] Spawn Distractor Signs
                (Utilities|FlowControl|Sequence
                  (:then_0
                    (Game|SpawnActorfromClass "/Game/Blueprints/PhoneBlueprint.PhoneBlueprint_C" (Variables|Default|GetDistractorsignSpawnTransform1) "Undefined" 0 0))
                  (:then_1
                    (Game|SpawnActorfromClass "/Game/Blueprints/LadderBlueprint.LadderBlueprint_C" (Variables|Default|GetDistractorsignSpawnTransform2) "Undefined" 0 0))
                  (:then_2
                    (Game|SpawnActorfromClass "/Game/Blueprints/FireextinguisherBlueprint.FireextinguisherBlueprint_C" (Variables|Default|GetDistractorsignSpawnTransform3) "Undefined" 0 0)))
                (else
                  (Development|PrintText "Distracting Signs OFF!" false))))
            (:then_2
              (if (Variables|/Game/Blueprints/LabyrinthGameInstance.LabyrinthGameInstance_C|GetFireAlarmEnabled _aslabyrinth_game_instance)
                (Development|PrintText "Fire Alarm ON!" false)
                ;[1 1 1] Spawn Fire Alarm
                (Utilities|FlowControl|Delay 1e+01)
                (Game|SpawnActorfromClass "/Game/Blueprints/FireAlarmSoundBlueprint.FireAlarmSoundBlueprint_C" (Math|Transform|MakeTransform "0, 0, 0") "Undefined" 0 0)
                (else
                  (Development|PrintText "Fire Alarm OFF!" false))))))
        (:CastFailed
          (Development|PrintString "CAST TO GAME INSTANCE FAILED!" false))))
    (:then_1
      ;[1 1 1] Placement of Random Object
      (switch Utilities|FlowControl|Switch|SwitchonObjectTypeEnum (Utilities|Enum|ByteToEnumObjectTypeEnum (Math|Conversions|ToByte(Integer) (Math|Random|RandomInteger 3)))
        (:NewEnumerator0
          (Game|SpawnActorfromClass "/Game/Blueprints/TrashcanBlueprint.TrashcanBlueprint_C" (Variables|Default|GetTrashcanAndFireSpawnEventTransform) "Undefined" 0 0))
        (:NewEnumerator1
          (Game|SpawnActorfromClass "/Game/Blueprints/SpiderV1Blueprint.SpiderV1Blueprint_C" (Variables|Default|GetSpiderSpawnEventTransform) "Undefined" 0 0))
        (:NewEnumerator2
          (Game|SpawnActorfromClass "/Game/Blueprints/FireBlueprint.FireBlueprint_C" (Variables|Default|GetTrashcanAndFireSpawnEventTransform) "Undefined" 0 0))))))

(fn ConstructionScript)