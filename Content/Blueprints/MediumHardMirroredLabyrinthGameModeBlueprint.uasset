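; Game mode Blueprint for the medium-hard mirrored labyrinth level, a child that supplies level-specific spawn placements to its parent game mode.
; On BeginPlay it calls SetParentVariables, then the parent's BeginPlay.
; SetParentVariables fills inherited transform variables with hardcoded locations, rotations and scales for trashcan, spider and fire events, plus escape and distractor signs.
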(event EventBeginPlay
  (CallFunction|SetParentVariables)
  (|CallParentFunction))

(event EventTick
  (params (DeltaSeconds :type Float%20%28single-precision%29)))

(fn ConstructionScript
  (|CallParentFunction))

(fn SetParentVariables
  ;[1 1 1] Set the variables of the parent blueprint which depend on the level
  (Utilities|FlowControl|Sequence
    (:then_0
      (Variables|Default|SetTrashcanSpawnEventTransform (Math|Transform|MakeTransform "-25.000000,-60.000000,25.000000" "0.000000,90.000000,90.000000" "5.000000,5.000000,5.000000")))
    (:then_1
      (Variables|Default|SetSpiderSpawnEventTransform (Math|Transform|MakeTransform "-40.000000,-60.000000,25.000000" "0.000000,90.000000,0.000000" "1.000000,1,1")))
    (:then_2
      (Variables|Default|SetEscapesignSpawnTransform1 (Math|Transform|MakeTransform "335.000000,1015.000000,170.000000" "0.000000,-180.000000,90.000000" "1.500000,1.500000,1.500000")))
    (:then_3
      (Variables|Default|SetEscapesignSpawnTransform2 (Math|Transform|MakeTransform "-300.000000,-555.000000,170.000000" "0.000000,-180.000000,90.000000" "1.500000,1.500000,1.500000")))
    (:then_4
      (Variables|Default|SetEscapesignSpawnTransform3 (Math|Transform|MakeTransform "0.000000,-50.000000,170.000000" "0.000000,-90.000000,90.000000" "1.500000,1.500000,1.500000")))
    (:then_5
      (Variables|Default|SetDistractorsignSpawnTransform1 (Math|Transform|MakeTransform "-270.000000,-555.000000,169.000000" "0.000000,0.000000,90.000000" "1.500000,1.500000,1.500000")))
    (:then_6
      (Variables|Default|SetDistractorsignSpawnTransform2 (Math|Transform|MakeTransform "-570.000000,950.000000,170.000000" "0.000000,-90.000000,90.000000" "1.500000,1.500000,1.500000")))
    (:then_7
      (Variables|Default|SetFireSpawnEventTransform (Math|Transform|MakeTransform "-25.000000,-60.000000,25.000000" "0.000000,90.000000,90.000000" "2.000000,2.000000,2.000000")))
    (:then_8
      (return))))